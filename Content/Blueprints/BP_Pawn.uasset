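; Pawn for a clicker game with a two-item shop: click power and passive income, bought with Score.
; UpdShop1 refreshes text components and colors buttons green or red by affordability, setting flags that gate the buy functions.
; Purchases raise the stat and double its cost, while AddScpersec adds passive income to Score.
; BeginPlay and click events are empty; the calls for scoring, buying and the looping income timer are disconnected.
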(event OnClicked(Mesh)
  (params (TouchedComponent :type Primitive%20Component%20Object%20Reference) (ButtonPressed :type Key%20Structure :default "None")))

(event OnClicked(ClickPowerBtn1)
  (params (TouchedComponent :type Primitive%20Component%20Object%20Reference) (ButtonPressed :type Key%20Structure :default "None")))

(event OnClicked(PasiveIncomeBtn1)
  (params (TouchedComponent :type Primitive%20Component%20Object%20Reference) (ButtonPressed :type Key%20Structure :default "None")))

(event EventBeginPlay)

(fn ConstructionScript)

(fn UpdShop1
  (bind _pasiveincomebtn1 (Variables|Default|GetPasiveIncomeBtn1))
  (bind _clickpowerbtn1 (Variables|Default|GetClickPowerBtn1))
  (Rendering|Components|TextRender|SetText (Variables|Default|GetClickPowerCostTxt1) (Utilities|Text|ToText(Integer) (Variables|Default|GetClickPowerCost1)))
  (Rendering|Components|TextRender|SetText (Variables|Default|GetClickPowerAddsTxt1) (Utilities|Text|ToText(Integer) (Variables|Default|GetClickPower)))
  (Rendering|Components|TextRender|SetText (Variables|Default|GetPassiveIncomeCostTxt1) (Utilities|Text|ToText(Integer) (Variables|Default|GetPassiveIncomeCost1)))
  (Rendering|Components|TextRender|SetText (Variables|Default|GetPassiveIncomeTxt1) (Utilities|Text|ToText(Integer) (Variables|Default|GetPassiveIncome1)))
  (Rendering|Components|TextRender|SetText (Variables|Default|GetScoreText) (Utilities|Text|ToText(Integer) (Variables|Default|GetScore)))
  (Utilities|FlowControl|Sequence
    (:then_0
      (bind _output_get (Variables|Default|SetClickPowerAwailable1 (>= (Variables|Default|GetScore) (Variables|Default|GetClickPowerCost1))))
      (if _output_get
        (Rendering|Material|SetMaterial _clickpowerbtn1 0 "/Game/Materials/MI_Green.MI_Green")
        (else
          (Rendering|Material|SetMaterial _clickpowerbtn1 0 "/Game/Materials/MI_Red.MI_Red"))))
    (:then_1
      (bind _output_get_2 (Variables|Default|SetPassiveIncomeAvailable1 (>= (Variables|Default|GetScore) (Variables|Default|GetPassiveIncomeCost1))))
      (if _output_get_2
        (Rendering|Material|SetMaterial _pasiveincomebtn1 0 "/Game/Materials/MI_Green.MI_Green")
        (else
          (Rendering|Material|SetMaterial _pasiveincomebtn1 0 "/Game/Materials/MI_Red.MI_Red"))))))

(fn BuyClPower
  (if (Variables|Default|GetClickPowerAwailable1)
    (Variables|Default|SetScore (- (Variables|Default|GetScore) (Variables|Default|GetClickPowerCost1)))
    (Variables|Default|SetClickPower (+ (Variables|Default|GetClickPower) (Variables|Default|GetClickPowerAdds1)))
    (Variables|Default|SetClickPowerCost1 (* (Variables|Default|GetClickPowerCost1) 2))
    (CallFunction|UpdShop1)))

(fn BuyScpersec
  (if (Variables|Default|GetPassiveIncomeAvailable1)
    (Variables|Default|SetScore (- (Variables|Default|GetScore) (Variables|Default|GetPassiveIncomeCost1)))
    (Variables|Default|SetPassiveIncome1 (+ (Variables|Default|GetPassiveIncome1) 1))
    (Variables|Default|SetPassiveIncomeCost1 (* (Variables|Default|GetPassiveIncomeCost1) 2))
    (CallFunction|UpdShop1)))

(fn AddScpersec
  (if (> (Variables|Default|GetPassiveIncome1) 0)
    (Variables|Default|SetScore (+ (Variables|Default|GetScore) (Variables|Default|GetPassiveIncome1)))
    (CallFunction|UpdShop1)))